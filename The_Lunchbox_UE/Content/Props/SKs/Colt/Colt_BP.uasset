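; Colt pistol prop that can be picked up by attaching to a socket, dropped with physics, and fired.
; Trigger and hammer pull amounts drive Colt_Anim_BP, with a click sound when the hammer first cocks.
; Shoot requires a cocked hammer and ammo, spawns a projectile with effects, updates the ammo text and resets the hammer.
; Tick repositions the ammo display when the mesh scale is mirrored to -1.
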(event `self.ReceiveTick`
  (params (DeltaSeconds :type "Float (single-precision)"))
  (if (== (`SceneComponent.RelativeScale3D` (`self.Colt_SK`)) (-1.0 -1.0 -1.0))
    (`SceneComponent.K2_SetRelativeTransform` (`self.AmmoCount`) (`self.LeftHandAmmoPos`) false false)))

(event `self.ReceiveBeginPlay`
  ;[1 1 1] Testing
)

(event `TriggerPull_0`
  (params (TriggerPull :type "Float (double-precision)"))
  (bind _output_get (set `self.TriggerPullAmt` TriggerPull))
  (bind _ascolt_anim_bp (cast `/Game/Animation/Colt/Colt_Anim_BP` (`SkeletalMeshComponent.GetAnimInstance` (`self.Colt_SK`))))
  (set `/Game/Animation/Colt/Colt_Anim_BP.triggerPull` _output_get _ascolt_anim_bp))

(event `HammerPulled_0`
  (params (HammerPull :type "Float (double-precision)"))
  (bind _output_get (set `self.HammerPullAmt` HammerPull))
  (bind _ascolt_anim_bp (cast `/Game/Animation/Colt/Colt_Anim_BP` (`SkeletalMeshComponent.GetAnimInstance` (`self.Colt_SK`))))
  (bind _output_get_2 (set `/Game/Animation/Colt/Colt_Anim_BP.hammerPull` _output_get _ascolt_anim_bp))
  (if (`self.hammerPulled`)
    _
    (elif (>= _output_get_2 0.6)
      (`GameplayStatics.SpawnSoundAtLocation` "/Game/Sound/gunClick.gunClick" (`SceneComponent.RelativeLocation` (`self.Arrow`)))
      (set `self.hammerPulled` true))))

(event `Shoot`
  (bind _arrow (`self.Arrow`))
  (bind _relativelocation (`SceneComponent.RelativeLocation` _arrow))
  ;[1 1 1] Shooting and ammo count
  (if (>= (`self.HammerPullAmt`) 0.6)
    (if (`self.hasAmmo`)
      (bind _returnvalue (`|SpawnActorFromClass` "/Game/Props/SKs/Colt/Bulet/FirstPersonProjectile.FirstPersonProjectile_C" (`KismetMathLibrary.MakeTransform` (.location (`SceneComponent.K2_GetComponentToWorld` (`self.Arrow`))) (.rotation (`SceneComponent.K2_GetComponentToWorld` (`self.Arrow`)))) "AdjustIfPossibleButAlwaysSpawn" "OverrideRootScale"))
      (set `self.ColtBullets` _returnvalue)
      (bind _output_get (set `self.CurrentAmmo` (- (`self.CurrentAmmo`) 1)))
      (set `self.hasAmmo` (> _output_get 0))
      (`TextRenderComponent.K2_SetText` (`self.AmmoCount`) (`KismetTextLibrary.Conv_IntToText` _output_get))
      (`GameplayStatics.PlaySoundAtLocation` "/Game/Sound/gunshot_08.gunshot_08" _relativelocation)
      (`GameplayStatics.SpawnEmitterAttached` "/Game/VRDemo_Assets/Emitters/Gun_Muzzle_A.Gun_Muzzle_A" _arrow "None" _relativelocation)
      (`GameplayStatics.SpawnSoundAtLocation` null _relativelocation)
      (bind _ascolt_anim_bp (cast `/Game/Animation/Colt/Colt_Anim_BP` (`SkeletalMeshComponent.GetAnimInstance` (`self.Colt_SK`))))
      (bind _output_get_2 (set `/Game/Animation/Colt/Colt_Anim_BP.hammerPull` -1.0 _ascolt_anim_bp))
      (set `self.HammerPullAmt` _output_get_2)
      (set `self.hammerPulled` false)
      (else
        (`KismetSystemLibrary.PrintString` "OUT OF AMMO YOU DUCK")))))

(event `/Game/Globals/VirtualReality/Blueprints/PickupActorInterface.Pickup`
  (params (AttachTo :type "SceneComponent Object Reference"))
  ;[1 1 1] Attaching and detaching COLT
  (`PrimitiveComponent.SetSimulatePhysics` (`self.Colt_SK`) false)
  (`self.K2_AttachToComponent` AttachTo "colt_Socket" "SnapToTarget" "SnapToTarget" "SnapToTarget" false))

(event `/Game/Globals/VirtualReality/Blueprints/PickupActorInterface.Drop`
  ;[1 1 1] Attaching and detaching COLT
  (`PrimitiveComponent.SetSimulatePhysics` (`self.Colt_SK`) true)
  (`self.K2_DetachFromActor` "KeepWorld" "KeepWorld" "KeepWorld"))

(fn `UserConstructionScript`)