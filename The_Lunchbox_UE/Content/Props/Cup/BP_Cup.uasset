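; BP_Cup is a pickup cup prop that changes color when tipped while held.
; Pickup disables physics and attaches it to the given parent; Drop detaches it and restores physics.
; While held, Tick compares roll and pitch against CupTipDegree, tinting a construction-script dynamic material green when tilted, red when upright.
; GrabBottle is empty, and level-sequence and walk-animation nodes are left unconnected.
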(event `GrabBottle`)

(event `/Game/Globals/VirtualReality/Blueprints/PickupActorInterface.Pickup`
  (params (AttachTo :type "SceneComponent Object Reference"))
  ;[1 1 1] Attaching and Detaching Cup
  (`PrimitiveComponent.SetSimulatePhysics` (`self.Cup`) false)
  (`self.K2_AttachToComponent` AttachTo "None" "KeepWorld" "KeepWorld" "KeepWorld")
  (set `self.HoldingCup` true))

(event `/Game/Globals/VirtualReality/Blueprints/PickupActorInterface.Drop`
  ;[1 1 1] Attaching and Detaching Cup
  (`PrimitiveComponent.SetSimulatePhysics` (`self.Cup`) true)
  (`self.K2_DetachFromActor` "KeepRelative")
  (set `self.HoldingCup` false)
  (set `self.PlayingAnim` false))

(event `self.ReceiveBeginPlay`)

(event `self.ReceiveTick`
  (params (DeltaSeconds :type "Float (single-precision)"))
  (bind _cuptipdegree (`self.CupTipDegree`))
  (bind (_returnvalue_roll _returnvalue_pitch) (`KismetMathLibrary.BreakRotator` (`SceneComponent.K2_GetComponentRotation` (`self.Cup`))))
  (bind _returnvalue (* _cuptipdegree -1.0))
  (if (`self.HoldingCup`)
    (if (or (> _returnvalue_roll _cuptipdegree) (> _returnvalue_pitch _cuptipdegree) (< _returnvalue_pitch _returnvalue) (< _returnvalue_roll _returnvalue))
      (`self.CupTilted`)
      (else
        (`self.CupUpright`)))))

(event `CupTilted`
  (`MaterialInstanceDynamic.SetVectorParameterValue` (`self.DM_CupREF`) "BaseColor" (struct :`R` 0.01436 :`G` 1.0 :`A` 1.0)))

(event `CupUpright`
  (`MaterialInstanceDynamic.SetVectorParameterValue` (`self.DM_CupREF`) "BaseColor" (struct :`R` 1.0 :`B` 0.089516 :`A` 1.0)))

(fn `UserConstructionScript`
  (bind _returnvalue (`PrimitiveComponent.CreateDynamicMaterialInstance` (`self.Cup`) 0 "/Game/Props/Cup/M_Cup.M_Cup"))
  (set `self.DM_CupREF` _returnvalue)
  (`SceneComponent.SetWorldScale3D` (`self.Cup`) (`self.CupScale`)))