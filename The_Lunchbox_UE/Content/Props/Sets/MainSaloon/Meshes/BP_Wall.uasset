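; BP_Wall is a resizable wall prop for the MainSaloon set, configured entirely in the construction script.
; It scales the Wall mesh by WallWidth and WallHeight and creates a dynamic M_Wall material instance.
; FacingPY, texture scale and horizontal and vertical shifts feed that material's parameters to control texture mapping.
; The event graph's rotation-based FacingPY detection is disconnected, and WallDepth is unused.
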(event `self.ReceiveTick`
  (params (DeltaSeconds :type "Float (single-precision)")))

(fn `UserConstructionScript`
  (bind _wall (`self.Wall`))
  (bind _wallmatref (`self.WallMatREF`))
  (bind _returnvalue (`PrimitiveComponent.CreateDynamicMaterialInstance` _wall 0 "/Game/Props/Sets/MainSaloon/Materials/M_Wall.M_Wall"))
  (set `self.WallMatREF` _returnvalue)
  (`SceneComponent.SetRelativeScale3D` _wall (`KismetMathLibrary.MakeVector` 1.0 (`self.Wall Width`) (`self.Wall Height`)))
  (`MaterialInstanceDynamic.SetScalarParameterValue` _wallmatref "MeshDirection" (`self.FacingPY`))
  (`MaterialInstanceDynamic.SetScalarParameterValue` _wallmatref "TextureScale" (`self.TextureScale`))
  (`MaterialInstanceDynamic.SetScalarParameterValue` _wallmatref "HorizontalShift" (`self.HorizontalShift`))
  (`MaterialInstanceDynamic.SetScalarParameterValue` _wallmatref "VerticalShift" (`self.VerticalShift`)))