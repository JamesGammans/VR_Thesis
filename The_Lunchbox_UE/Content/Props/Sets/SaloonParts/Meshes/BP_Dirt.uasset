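; BP_Dirt is a configurable saloon set prop that provides a resizable dirt surface built on a Floor mesh component.
; Its construction script scales the mesh by the wall depth, width and height variables, then creates a dynamic instance of M_Global on it.
; Exposed variables feed that material's texture, projection direction, scale, shift and rotation parameters, so each placed copy is textured independently.
; The event graph has no runtime logic.
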(event `self.ReceiveTick`
  (params (DeltaSeconds :type "Float (single-precision)")))

(fn `UserConstructionScript`
  (bind _floor (`self.Floor`))
  (bind _globalref_to_dirt (`self.GlobalREF_to_Dirt`))
  (bind _returnvalue (`PrimitiveComponent.CreateDynamicMaterialInstance` _floor 0 "/Game/Props/Sets/SaloonParts/Materials/M_Global.M_Global"))
  (set `self.GlobalREF_to_Dirt` _returnvalue)
  (`SceneComponent.SetRelativeScale3D` _floor (`KismetMathLibrary.MakeVector` (`self.Wall Depth`) (`self.Wall Width`) (`self.Wall Height`)))
  (`MaterialInstanceDynamic.SetTextureParameterValue` _globalref_to_dirt "MatTexture" (`self.MatTexture`))
  (`MaterialInstanceDynamic.SetScalarParameterValue` _globalref_to_dirt "MeshDirection_Z" (`self.Z_OnOff`))
  (`MaterialInstanceDynamic.SetScalarParameterValue` _globalref_to_dirt "MeshDirection_Y_X" (`self.X_or_Y`))
  (`MaterialInstanceDynamic.SetScalarParameterValue` _globalref_to_dirt "TextureScale" (`self.TextureScale`))
  (`MaterialInstanceDynamic.SetScalarParameterValue` _globalref_to_dirt "HorizontalShift" (`self.HorizontalShift`))
  (`MaterialInstanceDynamic.SetScalarParameterValue` _globalref_to_dirt "VerticalShift" (`self.VerticalShift`))
  (`MaterialInstanceDynamic.SetScalarParameterValue` _globalref_to_dirt "TextureRotation" (`self.TextureAngle`)))