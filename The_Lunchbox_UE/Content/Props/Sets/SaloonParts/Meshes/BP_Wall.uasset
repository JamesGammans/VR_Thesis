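; BP_Wall is a resizable wall piece for the saloon prop set, configured through its construction script.
; The script scales the Wall mesh by depth, width and height variables and creates a dynamic instance of M_Global on it.
; It passes facing, texture scale and horizontal and vertical shift variables to that material as scalar parameters.
; Event graph logic to derive FacingPY from wall rotation is unconnected, so it never runs.
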(event `self.ReceiveTick`
  (params (DeltaSeconds :type "Float (single-precision)")))

(fn `UserConstructionScript`
  (bind _wall (`self.Wall`))
  (bind _m_wallglobalref (`self.M_WallGlobalREF`))
  (bind _returnvalue (`PrimitiveComponent.CreateDynamicMaterialInstance` _wall 0 "/Game/Props/Sets/SaloonParts/Materials/M_Global.M_Global"))
  (set `self.M_WallGlobalREF` _returnvalue)
  (`SceneComponent.SetRelativeScale3D` _wall (`KismetMathLibrary.MakeVector` (`self.Wall Depth`) (`self.Wall Width`) (`self.Wall Height`)))
  (`MaterialInstanceDynamic.SetScalarParameterValue` _m_wallglobalref "MeshDirection_Y_X" (`self.FacingPY`))
  (`MaterialInstanceDynamic.SetScalarParameterValue` _m_wallglobalref "MeshDirection_Z" (`self.FacingPZ`))
  (`MaterialInstanceDynamic.SetScalarParameterValue` _m_wallglobalref "TextureScale" (`self.TextureScale`))
  (`MaterialInstanceDynamic.SetScalarParameterValue` _m_wallglobalref "HorizontalShift" (`self.HorizontalShift`))
  (`MaterialInstanceDynamic.SetScalarParameterValue` _m_wallglobalref "VerticalShift" (`self.VerticalShift`)))