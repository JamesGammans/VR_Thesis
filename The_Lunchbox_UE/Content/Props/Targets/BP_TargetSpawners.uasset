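; BP_TargetSpawners is a target-practice spawner that places BP_RedTarget actors at random points inside its Volume box.
; Each SpawnTargets call caches existing targets in MyTargets, then spawns one more until the CurrentTargets counter reaches ten.
; StartTargetPractice and BeginPlay are empty, and the looping spawn timer and delayed cleanup are unwired.
; DestroyTarget destroys an array element, but its loop over MyTargets is disconnected.
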(event Custom|SpawnTargets
  (bind _volume (Variables|Default|GetVolume))
  (bind _outactors (Actor|GetAllActorsOfClass "/Game/Props/Targets/BP_RedTarget.BP_RedTarget_C"))
  (bind _output_get (Variables|Default|SetMyTargets _outactors))
  (if (not (== (Variables|Default|GetCurrentTargets) 1e+01))
    (Game|SpawnActorfromClass "/Game/Props/Targets/BP_RedTarget.BP_RedTarget_C" (Math|Conversions|ToTransform(Vector) (Math|Random|RandomPointinBoundingBox (Transformation|GetWorldLocation _volume) (Components|Box|GetScaledBoxExtent _volume))) "Undefined" 0 0)
    (bind _result (Math|Float|IncrementFloat (Variables|Default|GetCurrentTargets))
      (:%20%20
        (Variables|Default|SetCurrentTargets _result)))))

(event Custom|DestroyTarget
  (Actor|DestroyActor (stale _array_element)))

(event Custom|StartTargetPractice)

(event EventBeginPlay)

(fn ConstructionScript)